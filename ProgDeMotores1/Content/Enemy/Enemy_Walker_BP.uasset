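; Walker enemy Blueprint that tracks its own health and has a melee attack event.
; Health starts at max on BeginPlay; GetDamage subtracts from it with clamping, then calls Die and destroys the actor at zero.
; MeleeAttack only calls PlayMontage on the mesh.
; A sphere-overlap damage block with debug drawing, gated by CanAttack, is disconnected and never runs.
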(event EventBeginPlay
  (Variables|Default|SetCurrentHealt (Variables|Default|GetMaxHealt)))

(event EventTick
  (params (DeltaSeconds :type Float%20%28single-precision%29)))

(event EventMeleeAttack
  (Animation|Montage|PlayMontage (Variables|Character|GetMesh) 0))

(event EventGetDamage
  (params (AmountOfDamage :type Float%20%28double-precision%29))
  (bind _output_get (Variables|Default|SetCurrentHealt (Math|Float|Clamp(Float) (- (Variables|Default|GetCurrentHealt) AmountOfDamage) 0.0 (Variables|Default|GetMaxHealt))))
  (if (== _output_get 0.0)
    (CallFunction|Die)
    (Actor|DestroyActor)))

(fn ConstructionScript)